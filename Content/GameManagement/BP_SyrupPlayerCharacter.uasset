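; BP_SyrupPlayerCharacter is a player character Blueprint that sets up the player's UI on BeginPlay.
; It adds the WBP_EnergyDisplay widget to the viewport and shows the mouse cursor for player controller 0.
; Unconnected draft nodes sketch cursor-trace click-to-move with an InteractInterface check and interaction radius, but never run and only print a placeholder instead of interacting.
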(event EventBeginPlay
  (bind _returnvalue (UserInterface|CreateWidget "/Game/UI/WBP_EnergyDisplay.WBP_EnergyDisplay_C"))
  (UserInterface|Viewport|AddtoViewport _returnvalue 0)
  (Variables|/Script/Engine.PlayerController|SetbShowMouseCursor (Game|GetPlayerController 0) true))

(event Input|MouseEvents|LeftMouseButton
  (params (Key :type Key%20Structure :default "None")))

(fn ConstructionScript)